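; BP_InkpotDemoGameMode is a game mode for an Inkpot story demo, with comments outlining display setup and story begin and end handling.
; BeginPlay, OnStoryBegin and OnStoryEnd are all empty.
; Unconnected nodes hold the intended logic: create a WBP_Display widget, set Game and UI input with a cursor, bind Inkpot story events, and show the story.
; As wired, none of that logic runs.
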(event Custom|Event%20OnStoryBegin
  (params (Story :type Inkpot%20Story%20Object%20Reference))
  ;[1 1 1] Display story when it begins
)

(event Custom|Event%20OnStoryEnd
  (params (Story :type Inkpot%20Story%20Object%20Reference))
  ;[1 1 1] Story End
)

(event EventBeginPlay
  ;[1 1 1] Setup display and control
)

(fn ConstructionScript)