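; Gameplay ability that fires a single projectile from the player character toward the mouse cursor.
; On activation it consumes mana, then spawns a BP_Parent_Projectile at the character's location, aimed using only X and Z of the deprojected cursor position.
; If the spawn succeeds, it copies the character's projectile damage onto the projectile, commits the cooldown and ends; a failed cast or spawn never reaches EndAbility.
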(event Ability|EventActivateAbility
  (bind _asbp_character (Utilities|Casting|CastToBP_Character (Ability|GetAvatarActorfromActorInfo)))
  (bind _output_get (Variables|Default|SetReference_Character _asbp_character))
  (Default|ConsumeMana _output_get)
  (bind _returnvalue (Game|SpawnActorfromClass "/Game/Blueprints/Projectiles/BP_Parent_Projectile.BP_Parent_Projectile_C" (Math|Transform|MakeTransform (Transformation|GetActorLocation _asbp_character) (Math|Rotator|FindLookatRotation (Transformation|GetActorLocation _asbp_character) (Math|Vector|MakeVector (.x (.WorldLocation (Game|Player|ConvertMouseLocationToWorldSpace (Variables|/Game/Player/BP_Character.BP_Character_C|GetReference_PlayerController (Variables|Default|GetReference_Character))))) 0.0 (.z (.WorldLocation (Game|Player|ConvertMouseLocationToWorldSpace (Variables|/Game/Player/BP_Character.BP_Character_C|GetReference_PlayerController (Variables|Default|GetReference_Character))))))) "1.000000,1.000000,1.000000") "AlwaysSpawn" "MultiplyWithRoot" 0 0))
  (Utilities|IsValid _returnvalue
    (:Is%20Valid
      (Variables|/Game/Blueprints/Projectiles/BP_Parent_Projectile.BP_Parent_Projectile_C|SetDamage _returnvalue (Variables|/Game/Player/BP_Character.BP_Character_C|GetProjectileDamage (Variables|Default|GetReference_Character)))
      (Ability|CommitAbilityCooldown false)
      (Ability|EndAbility))))