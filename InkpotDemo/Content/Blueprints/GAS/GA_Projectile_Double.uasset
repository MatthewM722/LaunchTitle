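; Gameplay ability that fires a double projectile from the player character toward the mouse cursor.
; On activation it consumes character mana and derives aim rotation from the deprojected mouse position's X and Z.
; It spawns two BP_Parent_Projectile actors, pitched up and down by InclineValue, passing each the character's damage and heart drop chance.
; It then commits the cooldown and ends the ability.
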(event Ability|EventActivateAbility
  (bind _asbp_character (Utilities|Casting|CastToBP_Character (Ability|GetAvatarActorfromActorInfo)))
  (bind _output_get (Variables|Default|SetReference_Character _asbp_character))
  (Default|ConsumeMana _output_get)
  (Variables|Default|SetRoll (.roll (Math|Rotator|FindLookatRotation (Transformation|GetActorLocation (Variables|Default|GetReference_Character)) (Math|Vector|MakeVector (.x (.WorldLocation (Game|Player|ConvertMouseLocationToWorldSpace (Variables|/Game/Player/BP_Character.BP_Character_C|GetReference_PlayerController (Variables|Default|GetReference_Character))))) 0.0 (.z (.WorldLocation (Game|Player|ConvertMouseLocationToWorldSpace (Variables|/Game/Player/BP_Character.BP_Character_C|GetReference_PlayerController (Variables|Default|GetReference_Character)))))))))
  (Variables|Default|SetPitch (.pitch (Math|Rotator|FindLookatRotation (Transformation|GetActorLocation (Variables|Default|GetReference_Character)) (Math|Vector|MakeVector (.x (.WorldLocation (Game|Player|ConvertMouseLocationToWorldSpace (Variables|/Game/Player/BP_Character.BP_Character_C|GetReference_PlayerController (Variables|Default|GetReference_Character))))) 0.0 (.z (.WorldLocation (Game|Player|ConvertMouseLocationToWorldSpace (Variables|/Game/Player/BP_Character.BP_Character_C|GetReference_PlayerController (Variables|Default|GetReference_Character)))))))))
  (Variables|Default|SetYaw (.yaw (Math|Rotator|FindLookatRotation (Transformation|GetActorLocation (Variables|Default|GetReference_Character)) (Math|Vector|MakeVector (.x (.WorldLocation (Game|Player|ConvertMouseLocationToWorldSpace (Variables|/Game/Player/BP_Character.BP_Character_C|GetReference_PlayerController (Variables|Default|GetReference_Character))))) 0.0 (.z (.WorldLocation (Game|Player|ConvertMouseLocationToWorldSpace (Variables|/Game/Player/BP_Character.BP_Character_C|GetReference_PlayerController (Variables|Default|GetReference_Character)))))))))
  (Utilities|FlowControl|Sequence
    (:then_0
      (bind _returnvalue (Game|SpawnActorfromClass "/Game/Blueprints/Projectiles/BP_Parent_Projectile.BP_Parent_Projectile_C" (Math|Transform|MakeTransform (Transformation|GetActorLocation (Variables|Default|GetReference_Character)) (Math|Rotator|MakeRotator (Variables|Default|GetRoll) (+ (Variables|Default|GetPitch) (Variables|Default|GetInclineValue)) (Variables|Default|GetYaw)) "1.000000,1.000000,1.000000") "AlwaysSpawn" "MultiplyWithRoot" 0 0))
      (Variables|/Game/Blueprints/Projectiles/BP_Parent_Projectile.BP_Parent_Projectile_C|SetDamage _returnvalue (Variables|/Game/Player/BP_Character.BP_Character_C|GetProjectileDamage (Variables|Default|GetReference_Character)))
      (Variables|/Game/Blueprints/Projectiles/BP_Parent_Projectile.BP_Parent_Projectile_C|SetHeartDropChance _returnvalue (Variables|/Game/Player/BP_Character.BP_Character_C|GetHeartDropChance (Variables|Default|GetReference_Character))))
    (:then_1
      (bind _returnvalue_2 (Game|SpawnActorfromClass "/Game/Blueprints/Projectiles/BP_Parent_Projectile.BP_Parent_Projectile_C" (Math|Transform|MakeTransform (Transformation|GetActorLocation (Variables|Default|GetReference_Character)) (Math|Rotator|MakeRotator (Variables|Default|GetRoll) (- (Variables|Default|GetPitch) (Variables|Default|GetInclineValue)) (Variables|Default|GetYaw)) "1.000000,1.000000,1.000000") "AlwaysSpawn" "MultiplyWithRoot" 0 0))
      (Variables|/Game/Blueprints/Projectiles/BP_Parent_Projectile.BP_Parent_Projectile_C|SetDamage _returnvalue_2 (Variables|/Game/Player/BP_Character.BP_Character_C|GetProjectileDamage (Variables|Default|GetReference_Character)))
      (Variables|/Game/Blueprints/Projectiles/BP_Parent_Projectile.BP_Parent_Projectile_C|SetHeartDropChance _returnvalue_2 (Variables|/Game/Player/BP_Character.BP_Character_C|GetHeartDropChance (Variables|Default|GetReference_Character))))
    (:then_2
      (Ability|CommitAbilityCooldown false)
      (Ability|EndAbility))))