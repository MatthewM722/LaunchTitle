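; GA_Hermes is a Gameplay Ability perk that boosts the avatar character's walk speed by a tenth.
; On activation it casts the avatar to BP_Character, raises MaxWalkSpeed on its CharacterMovement directly, then ends immediately.
; The change uses no Gameplay Effect and is never reverted here, so each activation compounds on the current speed.
; A failed cast stops execution before EndAbility is reached.
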(event Ability|EventActivateAbility
  (bind _asbp_character (Utilities|Casting|CastToBP_Character (Ability|GetAvatarActorfromActorInfo)))
  (Variables|Default|SetReference_Character _asbp_character)
  (Variables|/Script/Engine.CharacterMovementComponent|SetMaxWalkSpeed (Variables|/Script/Engine.Character|GetCharacterMovement (Variables|Default|GetReference_Character)) (+ (Variables|/Script/Engine.CharacterMovementComponent|GetMaxWalkSpeed (Variables|/Script/Engine.Character|GetCharacterMovement (Variables|Default|GetReference_Character))) (/ (Variables|/Script/Engine.CharacterMovementComponent|GetMaxWalkSpeed (Variables|/Script/Engine.Character|GetCharacterMovement (Variables|Default|GetReference_Character))) 1e+01)))
  (Ability|EndAbility))