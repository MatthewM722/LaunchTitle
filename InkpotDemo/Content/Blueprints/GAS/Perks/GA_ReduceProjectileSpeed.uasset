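; GA_ReduceProjectileSpeed is a Gameplay Ability perk that makes the character's projectiles slower but longer-ranged.
; On activation it casts the avatar actor to BP_Character, cuts ProjectileSpeed by a fifth and raises ProjectileRange by a fifth, then ends the ability.
; It edits the character's variables directly, so each activation compounds on the current values, and nothing in the graph reverts the change.
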(event Ability|EventActivateAbility
  (bind _asbp_character (Utilities|Casting|CastToBP_Character (Ability|GetAvatarActorfromActorInfo)))
  (bind _output_get (Variables|Default|SetReference_Character _asbp_character))
  (Variables|/Game/Player/BP_Character.BP_Character_C|SetProjectileSpeed _output_get (- (Variables|/Game/Player/BP_Character.BP_Character_C|GetProjectileSpeed _output_get) (/ (Variables|/Game/Player/BP_Character.BP_Character_C|GetProjectileSpeed _output_get) 5.0)))
  (Variables|/Game/Player/BP_Character.BP_Character_C|SetProjectileRange _output_get (+ (Variables|/Game/Player/BP_Character.BP_Character_C|GetProjectileRange _output_get) (/ (Variables|/Game/Player/BP_Character.BP_Character_C|GetProjectileRange _output_get) 5.0)))
  (Ability|EndAbility))