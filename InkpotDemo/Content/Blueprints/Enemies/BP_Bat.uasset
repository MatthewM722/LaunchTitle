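; BP_Bat is a flying enemy that patrols horizontally with a vertical bob and can drop projectiles.
; A Timeline drives the capsule from its start position, reversing and flipping facing at each end via a FlipFlop.
; Looping timers spawn BP_BatProjectile below it and damage overlapping BPI_EnemyInterface actors.
; ACEnemyComponent handles incoming damage; successful hits pause movement for the stun duration, and stun blocks new shots and overlap damage.
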(event OnComponentBeginOverlap(CapsuleComponent)
  (params (OverlappedComponent :type Primitive%20Component%20Object%20Reference) (OtherActor :type Actor%20Object%20Reference) (OtherComp :type Primitive%20Component%20Object%20Reference) (OtherBodyIndex :type Integer) (bFromSweep :type Boolean) (SweepResult :type Hit%20Result%20Structure%20%28by%20ref%29))
  ;[1 1 1] Overlap Damage To Player
  (if (not (Variables|/Game/Blueprints/AC_EnemyComponent.AC_EnemyComponent_C|GetStunned (Variables|Default|GetAC_EnemyComponent)))
    (Utilities|IsValid OtherActor
      (:Is%20Valid
        (if (Utilities|DoesObjectImplementInterface OtherActor "/Game/Blueprints/BPI_EnemyInterface.BPI_EnemyInterface_C")
          (Utilities|Time|SetTimerbyEvent (delegate Custom|Hit) 0.1 true))))))

(event OnComponentEndOverlap(CapsuleComponent)
  (params (OverlappedComponent :type Primitive%20Component%20Object%20Reference) (OtherActor :type Actor%20Object%20Reference) (OtherComp :type Primitive%20Component%20Object%20Reference) (OtherBodyIndex :type Integer))
  ;[1 1 1] Overlap Damage To Player
  (Utilities|Time|ClearTimerbyFunctionName 0 "Hit"))

(event Custom|Hit
  ;[1 1 1] Overlap Damage To Player
  (Class|BPIEnemyInterface|DamageTarget(Message) (stale OnComponentBeginOverlap(CapsuleComponent) OtherActor) 1.0 "NewEnumerator0"))

(event Custom|Stop
  (bind _initiallocation (Variables|Default|GetInitialLocation))
  ;[1 1 1] Movement
  (bind (_direction _horizontal_alpha _vertical_alpha) (Timeline|Timeline Stop)
    (:Update
      (Transformation|SetWorldLocation (Variables|Collision|GetCapsuleComponent) (Math|Vector|MakeVector (Math|Float|Lerp (.x _initiallocation) (+ (.x _initiallocation) (Variables|Default|GetHorizontal%20Distance)) _horizontal_alpha) (.y (Variables|Default|GetInitialLocation)) (Math|Float|Lerp (.z _initiallocation) (+ (.z _initiallocation) 2e+01) (* _vertical_alpha -1.0))) false false))
    (:Finished
      (Utilities|FlowControl|FlipFlop
        (:A
          (Variables|Default|SetRight true))
        (:B
          (Variables|Default|SetRight false)))
      (if (Variables|Default|GetRight)
        (CallFunction|TurnRight)
        (Timeline|Timeline Play)
        (else
          (CallFunction|TurnLeft)
          (Timeline|Timeline Reverse))))))

(event Custom|Resume
  (bind _initiallocation (Variables|Default|GetInitialLocation))
  ;[1 1 1] Movement
  (if (Variables|Default|GetRight) :!label _label
    (CallFunction|TurnRight)
    (bind (_direction _horizontal_alpha _vertical_alpha) (Timeline|Timeline Play)
      (:Update
        (Transformation|SetWorldLocation (Variables|Collision|GetCapsuleComponent) (Math|Vector|MakeVector (Math|Float|Lerp (.x _initiallocation) (+ (.x _initiallocation) (Variables|Default|GetHorizontal%20Distance)) _horizontal_alpha) (.y (Variables|Default|GetInitialLocation)) (Math|Float|Lerp (.z _initiallocation) (+ (.z _initiallocation) 2e+01) (* _vertical_alpha -1.0))) false false))
      (:Finished
        (Utilities|FlowControl|FlipFlop
          (:A
            (Variables|Default|SetRight true)
            (goto _label))
          (:B
            (Variables|Default|SetRight false)
            (goto _label)))))
    (else
      (CallFunction|TurnLeft)
      (Timeline|Timeline Reverse))))

(event Custom|Rock%20Throw
  (bind _returnvalue (Transformation|GetActorLocation))
  ;[1 1 1] Shooting
  (if (not (Variables|/Game/Blueprints/AC_EnemyComponent.AC_EnemyComponent_C|GetStunned (Variables|Default|GetAC_EnemyComponent)))
    (Game|SpawnActorfromClass "/Game/Blueprints/Projectiles/BP_BatProjectile.BP_BatProjectile_C" (Math|Transform|MakeTransform (Math|Vector|MakeVector (.x _returnvalue) (.y _returnvalue) (- (.z _returnvalue) 3e+01)) "0, 0, 0" "1.200000,1.200000,1.200000") "Undefined" "MultiplyWithRoot" 0 0)))

(event EventBeginPlay
  (Utilities|FlowControl|Sequence
    (:then_0
      ;[1 1 1] Movement
      (Variables|Default|SetInitialLocation (Transformation|GetWorldLocation (Variables|Collision|GetCapsuleComponent)))
      (if (Variables|Default|GetRight) :!label _label
        (CallFunction|TurnRight)
        (bind (_direction _horizontal_alpha _vertical_alpha) (Timeline|Timeline Play)
          (:Update
            (Transformation|SetWorldLocation (Variables|Collision|GetCapsuleComponent) (Math|Vector|MakeVector (Math|Float|Lerp (.x (Variables|Default|GetInitialLocation)) (+ (.x (Variables|Default|GetInitialLocation)) (Variables|Default|GetHorizontal%20Distance)) _horizontal_alpha) (.y (Variables|Default|GetInitialLocation)) (Math|Float|Lerp (.z (Variables|Default|GetInitialLocation)) (+ (.z (Variables|Default|GetInitialLocation)) 2e+01) (* _vertical_alpha -1.0))) false false))
          (:Finished
            (Utilities|FlowControl|FlipFlop
              (:A
                (Variables|Default|SetRight true)
                (goto _label))
              (:B
                (Variables|Default|SetRight false)
                (goto _label)))))
        (else
          (CallFunction|TurnLeft)
          (Timeline|Timeline Reverse))))
    (:then_1
      ;[1 1 1] Shooting
      (if (Variables|Default|GetShoots)
        (Utilities|Time|SetTimerbyEvent (delegate Custom|Rock%20Throw) (/ 1.0 (Variables|Default|GetRateOfFire)) true)))))

(event EventDamageTarget
  (params (Amount :type Float%20%28double-precision%29) (DamageType :type ENUM_DamageTypes%20Enum :default "NewEnumerator0"))
  ;[1 1 1] Damaged
  (bind _wasstunned_ (Default|ACDamageTarget (Variables|Default|GetAC_EnemyComponent) Amount DamageType))
  (if _wasstunned_
    (CallFunction|Stop)
    (Utilities|FlowControl|Delay (Variables|/Game/Blueprints/AC_EnemyComponent.AC_EnemyComponent_C|GetStunDuration (Variables|Default|GetAC_EnemyComponent)))
    (CallFunction|Resume)))

(fn ConstructionScript)

(fn TurnLeft
  (Transformation|SetActorRotation "0.000000,180.000000,0.000000"))

(fn TurnRight
  (Transformation|SetActorRotation "0, 0, 0"))