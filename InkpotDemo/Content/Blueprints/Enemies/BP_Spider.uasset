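; Spider enemy that acts as a turret, deals contact damage through its Box, and drops a health pickup on death.
; BeginPlay scales the Sphere by Range, and actor overlaps open or close a firing gate.
; A looping timer at RateOfFire spawns spider projectiles aimed at the overlapping BP_Character's current position.
; Path-prediction aiming is present but disconnected and never runs.
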(event OnComponentBeginOverlap(Box)
  (params (OverlappedComponent :type Primitive%20Component%20Object%20Reference) (OtherActor :type Actor%20Object%20Reference) (OtherComp :type Primitive%20Component%20Object%20Reference) (OtherBodyIndex :type Integer) (bFromSweep :type Boolean) (SweepResult :type Hit%20Result%20Structure%20%28by%20ref%29))
  (Class|BPIEnemyInterface|DamageTarget(Message) OtherActor 1.0 0.0))

(event Custom|Turret
  (bind _returnvalue (Transformation|GetActorLocation))
  (Utilities|FlowControl|Gate true
    (:Exit
      (Game|SpawnActorfromClass "/Game/Blueprints/Projectiles/BP_Child_SpiderProjectile.BP_Child_SpiderProjectile_C" (Math|Transform|MakeTransform _returnvalue (Math|Rotator|FindLookatRotation _returnvalue (Transformation|GetActorLocation (Variables|Default|GetReference_Character))) "1.000000,1.000000,1.000000") "Undefined" "MultiplyWithRoot" 0 0))))

(event Custom|CloseGate
  (bind _returnvalue (Transformation|GetActorLocation))
  (Utilities|FlowControl|Gate true) ; enters at Close
)

(event Custom|OpenGate
  (bind _returnvalue (Transformation|GetActorLocation))
  (Utilities|FlowControl|Gate true) ; enters at Open
)

(event EventDamageTarget
  (params (Amount :type Float%20%28double-precision%29) (HeartDropChance :type Float%20%28double-precision%29))
  (Variables|Default|SetHealth (- (Variables|Default|GetHealth) Amount))
  (if (<= (Variables|Default|GetHealth) 0.0)
    (Game|SpawnActorfromClass "/Game/Blueprints/BP_HealthPickup.BP_HealthPickup_C" (Math|Transform|MakeTransform (Transformation|GetWorldLocation (Variables|Default|GetPlane)) "0, 0, 0" "1.000000,1.000000,1.000000") "AlwaysSpawn" "MultiplyWithRoot" 0 0)
    (Actor|DestroyActor)))

(event EventTick
  (params (DeltaSeconds :type Float%20%28single-precision%29))
  ;[1 1 1] Path Prediction
)

(event Collision|EventActorBeginOverlap
  (params (OtherActor :type Actor%20Object%20Reference))
  (CallFunction|OpenGate)
  (bind _asbp_character (Utilities|Casting|CastToBP_Character OtherActor))
  (Variables|Default|SetReference_Character _asbp_character)
  (Utilities|Time|SetTimerbyEvent (delegate Custom|Turret) (/ 1.0 (Variables|Default|GetRateOfFire)) true))

(event Collision|EventActorEndOverlap
  (params (OtherActor :type Actor%20Object%20Reference))
  (Utilities|Casting|CastToBP_Character OtherActor)
  (CallFunction|CloseGate))

(event EventBeginPlay
  (Transformation|SetRelativeScale3D (Variables|Default|GetSphere) (Math|Conversions|ToVector(Float) (Variables|Default|GetRange))))

(fn ConstructionScript)