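; BP_BatProjectile is a 2D projectile that damages what it overlaps.
; On spawn it picks a random sprite from its list and launches its box downward with a velocity-change impulse and slight random horizontal spread.
; When the box begins an overlap, it sends a damage message to the other actor and destroys itself, with no filtering on what was hit.
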(event OnComponentBeginOverlap(Box)
  (params (OverlappedComponent :type Primitive%20Component%20Object%20Reference) (OtherActor :type Actor%20Object%20Reference) (OtherComp :type Primitive%20Component%20Object%20Reference) (OtherBodyIndex :type Integer) (bFromSweep :type Boolean) (SweepResult :type Hit%20Result%20Structure%20%28by%20ref%29))
  ;[1 1 1] Hit
  (Class|BPIEnemyInterface|DamageTarget(Message) OtherActor 1.0 "NewEnumerator0")
  (Actor|DestroyActor))

(event EventBeginPlay
  ;[1 1 1] Random bounce on spawn
  (Rendering|Components|Sprite|SetSprite (Variables|Default|GetPaperSprite) (.OutItem (Utilities|Array|Random (Variables|Default|GetSpriteList))))
  (Physics|AddImpulse (Variables|Default|GetBox) (* (Math|Vector|MakeVector (Math|Random|RandomFloatinRange -0.5 0.5) 0.0 -1.0) 2e+02) "None" true))

(fn ConstructionScript)