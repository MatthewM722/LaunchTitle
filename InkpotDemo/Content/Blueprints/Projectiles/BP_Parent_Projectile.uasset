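; Base projectile Blueprint that damages enemies and bursts on overlap, with an optional radial impulse.
; Construction script applies speed and lifespan to the projectile.
; Overlapping an enemy-interface actor calls the hit notification, sends damage, spawns the burst and destroys the projectile.
; Other overlaps burst and destroy it, first firing RadialForce if it is an impulse projectile and the player is falling.
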(event OnComponentBeginOverlap(Collision)
  (params (OverlappedComponent :type Primitive%20Component%20Object%20Reference) (OtherActor :type Actor%20Object%20Reference) (OtherComp :type Primitive%20Component%20Object%20Reference) (OtherBodyIndex :type Integer) (bFromSweep :type Boolean) (SweepResult :type Hit%20Result%20Structure%20%28by%20ref%29))
  (if (Utilities|DoesObjectImplementInterface OtherActor "/Game/Blueprints/BPI_EnemyInterface.BPI_EnemyInterface_C")
    (Utilities|FlowControl|Sequence
      (:then_0
        (Default|CallProjectileHit)
        (Class|BPIEnemyInterface|DamageTarget(Message) OtherActor (Variables|Default|GetDamage) "NewEnumerator0")
        (Niagara|SpawnSystematLocation "/Game/Assets/NiagaraSystems/ProjectileBurst.ProjectileBurst" (Transformation|GetActorLocation)))
      (:then_2
        (Actor|DestroyActor)))
    (else
      (if (Variables|Default|GetImpulseProjectile)
        (bind _asbp_character (Utilities|Casting|CastToBP_Character (Game|GetPlayerCharacter 0)))
        (if (AI|Components|NavMovement|IsFalling (Variables|/Script/Engine.Character|GetCharacterMovement _asbp_character))
          (CallFunction|Impulse)))
      (Niagara|SpawnSystematLocation "/Game/Assets/NiagaraSystems/ProjectileBurst.ProjectileBurst" (Transformation|GetActorLocation))
      (Actor|DestroyActor))))

(event EventBeginPlay)

(fn ConstructionScript
  (Variables|/Script/Engine.ProjectileMovementComponent|SetMaxSpeed (Variables|Default|GetProjectileMovement) (Variables|Default|GetSpeed))
  (Variables|/Script/Engine.ProjectileMovementComponent|SetInitialSpeed (Variables|Default|GetProjectileMovement) (Variables|Default|GetSpeed))
  (Actor|SetLifeSpan (Variables|Default|GetDuration%20/%20Range)))

(fn Impulse
  (Class|RadialForceComponent|FireImpulse (Variables|Default|GetRadialForce)))