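; Enemy actor component that handles health, armour, stun and death drops.
; Normal damage only hurts unarmoured enemies, while armour-breaking hits wear down armour or health and stun survivors.
; Depleted armour makes the enemy vulnerable and notifies the owner by interface, and stuns are followed by brief immunity.
; Death always drops mana, drops health by the player's chance, and destroys the owner unless chain damage is active.
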(event Custom|Stun
  (if (not (Variables|Default|GetStunImmunity))
    (Variables|Default|SetStunned true)
    (Utilities|FlowControl|Delay (Variables|Default|GetStunDuration))
    (Variables|Default|SetStunned false)
    (Variables|Default|SetStunImmunity true)
    (Utilities|FlowControl|Delay 2.0)
    (Variables|Default|SetStunImmunity false)))

(event EventBeginPlay
  (bind _output_get (Variables|Default|SetVulnerable (not (> (Variables|Default|GetArmour) 0.0))))
  (if _output_get
    _))

(fn Death
  (bind _asbp_character (Utilities|Casting|CastToBP_Character (Game|GetPlayerCharacter 0)))
  (LocalVariables|SetHeartDropChance (Variables|/Game/Player/BP_Character.BP_Character_C|GetHeartDropChance _asbp_character))
  (LocalVariables|SetChainDamageActive (Variables|/Game/Player/BP_Character.BP_Character_C|GetChainDamageActive _asbp_character))
  (if (<= (Math|Random|RandomFloatinRange 0.0 1e+02) (LocalVariables|GetHeartDropChance))
    (Game|SpawnActorfromClass "/Game/Blueprints/Pickups/BP_HealthPickup.BP_HealthPickup_C" (Math|Transform|MakeTransform (Transformation|GetWorldLocation (Variables|/Script/Engine.Actor|GetRootComponent (Components|GetOwner))) "0, 0, 0" "1.000000,1.000000,1.000000") "AlwaysSpawn" "MultiplyWithRoot" 0 0))
  (Game|SpawnActorfromClass "/Game/Blueprints/Pickups/BP_ManaPickup.BP_ManaPickup_C" (Math|Transform|MakeTransform (Transformation|GetWorldLocation (Variables|/Script/Engine.Actor|GetRootComponent (Components|GetOwner))) "0, 0, 0" "1.000000,1.000000,1.000000") "AlwaysSpawn" "MultiplyWithRoot" 0 0)
  (if (not (LocalVariables|GetChainDamageActive))
    (Actor|DestroyActor (Components|GetOwner))))

(fn BreakArmour
  (Variables|Default|SetVulnerable true)
  (Class|BPIEnemyInterface|BPIBreakArmour(Message) (Components|GetOwner)))

(fn ACDamageTarget
  (params (Amount :type Float%20%28double-precision%29) (DamageType :type ENUM_DamageTypes%20Enum :default "NewEnumerator0"))
  (switch Utilities|FlowControl|Switch|SwitchonENUM_DamageTypes DamageType
    (:NewEnumerator0
      (if (Variables|Default|GetVulnerable)
        (Variables|Default|SetHealth (- (Variables|Default|GetHealth) Amount))
        (if (<= (Variables|Default|GetHealth) 0.0)
          (CallFunction|Death))
        (else
          (Development|PrintString "Damage Blocked")))
      (return false))
    (:NewEnumerator1
      (if (Variables|Default|GetVulnerable)
        (Variables|Default|SetHealth (- (Variables|Default|GetHealth) Amount))
        (if (<= (Variables|Default|GetHealth) 0.0)
          (CallFunction|Death)
          (return false)
          (else
            (CallFunction|Stun)
            (return true)))
        (else
          (Variables|Default|SetArmour (- (Variables|Default|GetArmour) Amount))
          (CallFunction|Stun)
          (if (<= (Variables|Default|GetArmour) 0.0)
            (CallFunction|BreakArmour))
          (return true))))))