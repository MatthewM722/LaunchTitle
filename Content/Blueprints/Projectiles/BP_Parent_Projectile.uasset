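; Parent projectile Blueprint that damages enemies on hit and destroys itself on any impact.
; On hit, targets implementing BPI_EnemyInterface receive a damage message carrying Damage and a heart drop chance, after a CallProjectileHit call.
; Other hits optionally fire a RadialForce impulse when ImpulseProjectile is set, before the actor is destroyed.
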(event Collision|EventHit
  (params (MyComp :type Primitive%20Component%20Object%20Reference) (Other :type Actor%20Object%20Reference) (OtherComp :type Primitive%20Component%20Object%20Reference) (bSelfMoved :type Boolean) (HitLocation :type Vector :default "0, 0, 0") (HitNormal :type Vector :default "0, 0, 0") (NormalImpulse :type Vector :default "0, 0, 0") (Hit :type Hit%20Result%20Structure%20%28by%20ref%29))
  (if (Utilities|DoesObjectImplementInterface Other "/Game/Blueprints/BPI_EnemyInterface.BPI_EnemyInterface_C")
    (Default|CallProjectileHit)
    (Class|BPIEnemyInterface|DamageTarget(Message) Other (Variables|Default|GetDamage) (Variables|Default|GetHeartDropChance))
    (Actor|DestroyActor)
    (else
      (if (Variables|Default|GetImpulseProjectile)
        (CallFunction|Impulse))
      (Actor|DestroyActor))))

(fn ConstructionScript)

(fn Impulse
  (Class|RadialForceComponent|FireImpulse (Variables|Default|GetRadialForce)))