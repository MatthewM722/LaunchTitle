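; BP_HealthPickup is a health pickup that pops upward on spawn, homes in on the player, then restores health.
; BeginPlay gives the Box an upward impulse with random X drift.
; The first Sphere overlap passes a DoOnce, and if it is BP_Character, stores it and plays a timeline lerping the Box toward its capsule.
; Any Box overlap calls IncreaseCurrentHealth on the stored character and destroys the pickup.
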(event OnComponentBeginOverlap(Sphere)
  (params (OverlappedComponent :type Primitive%20Component%20Object%20Reference) (OtherActor :type Actor%20Object%20Reference) (OtherComp :type Primitive%20Component%20Object%20Reference) (OtherBodyIndex :type Integer) (bFromSweep :type Boolean) (SweepResult :type Hit%20Result%20Structure%20%28by%20ref%29))
  ;[1 1 1] Overlaps the player
  (Utilities|FlowControl|DoOnce false
    (:Completed
      (bind _asbp_character (Utilities|Casting|CastToBP_Character OtherActor))
      (Variables|Default|SetReference_Character _asbp_character)
      (CallFunction|StartTracking))))

(event OnComponentBeginOverlap(Box)
  (params (OverlappedComponent :type Primitive%20Component%20Object%20Reference) (OtherActor :type Actor%20Object%20Reference) (OtherComp :type Primitive%20Component%20Object%20Reference) (OtherBodyIndex :type Integer) (bFromSweep :type Boolean) (SweepResult :type Hit%20Result%20Structure%20%28by%20ref%29))
  ;[1 1 1] Collected
  (Default|IncreaseCurrentHealth (Variables|Default|GetReference_Character))
  (Actor|DestroyActor))

(event Custom|StartTracking
  ;[1 1 1] Tracks the player's movement
  (bind _newtrack_0 (Timeline|PlayerTrack Play)
    (:Update
      (Transformation|SetWorldLocation (Variables|Default|GetBox) (Math|Vector|Lerp(Vector) (Transformation|GetWorldLocation (Variables|Default|GetBox)) (Transformation|GetWorldLocation (Variables|/Script/Engine.Character|GetCapsuleComponent (Variables|Default|GetReference_Character))) _newtrack_0) false false))))

(event EventBeginPlay
  ;[1 1 1] Random bounce on spawn
  (Physics|AddImpulse (Variables|Default|GetBox) (* (Math|Vector|MakeVector (Math|Random|RandomFloatinRange -0.5 0.5) 0.0 1.0) 2e+02) "None" true))

(fn ConstructionScript)