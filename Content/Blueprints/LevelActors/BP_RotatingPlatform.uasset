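; BP_RotatingPlatform is a level actor that swings back and forth around a single axis at constant speed.
; BeginPlay starts an endless Delay loop that flips the RotatingMovement component's RotationRate sign, with no Tick or timeline.
; The first leg lasts half as long as later ones, centring the swing on the starting orientation.
; The Invert flag selects a mirrored sequence that starts in the opposite direction.
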(event EventBeginPlay
  (if (Variables|Default|GetInvert)
    (Variables|/Script/Engine.RotatingMovementComponent|SetRotationRate (Variables|Default|GetRotatingMovement) "-20.000000,0.000000,0.000000")
    (Utilities|FlowControl|Delay 1.0)
    (Variables|/Script/Engine.RotatingMovementComponent|SetRotationRate (Variables|Default|GetRotatingMovement) "20.000000,0.000000,0.000000" :!label _label)
    (Utilities|FlowControl|Delay 2.0)
    (Variables|/Script/Engine.RotatingMovementComponent|SetRotationRate (Variables|Default|GetRotatingMovement) "-20.000000,0.000000,0.000000")
    (Utilities|FlowControl|Delay 2.0)
    (goto _label)
    (else
      (Variables|/Script/Engine.RotatingMovementComponent|SetRotationRate (Variables|Default|GetRotatingMovement) "20.000000,0.000000,0.000000")
      (Utilities|FlowControl|Delay 1.0)
      (Variables|/Script/Engine.RotatingMovementComponent|SetRotationRate (Variables|Default|GetRotatingMovement) "-20.000000,0.000000,0.000000" :!label _label_2)
      (Utilities|FlowControl|Delay 2.0)
      (Variables|/Script/Engine.RotatingMovementComponent|SetRotationRate (Variables|Default|GetRotatingMovement) "20.000000,0.000000,0.000000")
      (Utilities|FlowControl|Delay 2.0)
      (goto _label_2))))

(fn ConstructionScript)