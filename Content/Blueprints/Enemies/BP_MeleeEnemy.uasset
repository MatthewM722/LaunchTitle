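; Melee enemy Blueprint that deals contact damage to actors entering its Box and can itself be damaged and killed.
; Box begin overlap starts a fast looping timer that sends DamageTarget messages to the overlapping actor, and end overlap pauses it by function name.
; Incoming DamageTarget calls subtract from Health and destroy the enemy once it reaches zero.
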(event OnComponentBeginOverlap(Box)
  (params (OverlappedComponent :type Primitive%20Component%20Object%20Reference) (OtherActor :type Actor%20Object%20Reference) (OtherComp :type Primitive%20Component%20Object%20Reference) (OtherBodyIndex :type Integer) (bFromSweep :type Boolean) (SweepResult :type Hit%20Result%20Structure%20%28by%20ref%29))
  (Utilities|Time|SetTimerbyEvent (delegate Custom|Hit) 0.1 true))

(event OnComponentEndOverlap(Box)
  (params (OverlappedComponent :type Primitive%20Component%20Object%20Reference) (OtherActor :type Actor%20Object%20Reference) (OtherComp :type Primitive%20Component%20Object%20Reference) (OtherBodyIndex :type Integer))
  (Class|KismetSystemLibrary|PauseTimer 0 "Hit"))

(event Custom|Hit
  (Class|BPIEnemyInterface|DamageTarget(Message) (stale OnComponentBeginOverlap(Box) OtherActor) 1.0))

(event EventDamageTarget
  (params (Amount :type Float%20%28double-precision%29))
  (Variables|Default|SetHealth (- (Variables|Default|GetHealth) Amount))
  (if (<= (Variables|Default|GetHealth) 0.0)
    (Actor|DestroyActor)))

(fn ConstructionScript)