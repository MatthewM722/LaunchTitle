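; BP_Spider is an enemy turret that fires projectiles at the player character within its range and is destroyed when damage depletes its health.
; BeginPlay scales the detection sphere by Range.
; A character overlap starts a looping fire-rate timer that spawns BP_Projectile aimed at the character's current position, through a Gate that overlaps open and character exit closes.
; A path-prediction aiming block exists but is disconnected.
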(event Custom|Turret
  (bind _returnvalue (Transformation|GetActorLocation))
  (Utilities|FlowControl|Gate true
    (:Exit
      (Game|SpawnActorfromClass "/Game/Blueprints/BP_Projectile.BP_Projectile_C" (Math|Transform|MakeTransform _returnvalue (Math|Rotator|FindLookatRotation _returnvalue (Transformation|GetActorLocation (Variables|Default|GetReference_Character))) "1.000000,1.000000,1.000000") "Undefined" "MultiplyWithRoot" 0 0))))

(event Custom|CloseGate
  (bind _returnvalue (Transformation|GetActorLocation))
  (Utilities|FlowControl|Gate true) ; enters at Close
)

(event Custom|OpenGate
  (bind _returnvalue (Transformation|GetActorLocation))
  (Utilities|FlowControl|Gate true) ; enters at Open
)

(event Custom|DamageTarget_1
  (params (Amount :type Float%20%28double-precision%29))
  (Variables|Default|SetHealth (- (Variables|Default|GetHealth) Amount))
  (if (<= (Variables|Default|GetHealth) 0.0)
    (Actor|DestroyActor)))

(event EventTick
  (params (DeltaSeconds :type Float%20%28single-precision%29))
  ;[1 1 1] Path Prediction
)

(event Collision|EventActorBeginOverlap
  (params (OtherActor :type Actor%20Object%20Reference))
  (CallFunction|OpenGate)
  (bind _asbp_character (Utilities|Casting|CastToBP_Character OtherActor))
  (Variables|Default|SetReference_Character _asbp_character)
  (Utilities|Time|SetTimerbyEvent (delegate Custom|Turret) (/ 1.0 (Variables|Default|GetRateOfFire)) true))

(event Collision|EventActorEndOverlap
  (params (OtherActor :type Actor%20Object%20Reference))
  (Utilities|Casting|CastToBP_Character OtherActor)
  (CallFunction|CloseGate))

(event EventBeginPlay
  (Transformation|SetRelativeScale3D (Variables|Default|GetSphere) (Math|Conversions|ToVector(Float) (Variables|Default|GetRange))))

(fn ConstructionScript)