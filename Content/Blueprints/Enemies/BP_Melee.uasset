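; BP_Melee is a patrolling melee enemy that damages actors it touches and can be killed.
; It walks forward every tick, turning around when its wall detector begins an overlap or its floor detector ends one.
; Its Box starts a looping timer that repeatedly damages overlapping BPI_EnemyInterface actors until an overlap ends.
; Incoming damage reduces Health; death rolls the attacker-supplied chance to spawn BP_HealthPickup, then destroys the actor.
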(event OnComponentBeginOverlap(Box)
  (params (OverlappedComponent :type Primitive%20Component%20Object%20Reference) (OtherActor :type Actor%20Object%20Reference) (OtherComp :type Primitive%20Component%20Object%20Reference) (OtherBodyIndex :type Integer) (bFromSweep :type Boolean) (SweepResult :type Hit%20Result%20Structure%20%28by%20ref%29))
  (if (Utilities|DoesObjectImplementInterface OtherActor "/Game/Blueprints/BPI_EnemyInterface.BPI_EnemyInterface_C")
    (Utilities|Time|SetTimerbyEvent (delegate Custom|Hit) 0.1 true)))

(event OnComponentEndOverlap(Box)
  (params (OverlappedComponent :type Primitive%20Component%20Object%20Reference) (OtherActor :type Actor%20Object%20Reference) (OtherComp :type Primitive%20Component%20Object%20Reference) (OtherBodyIndex :type Integer))
  (Utilities|Time|ClearTimerbyFunctionName 0 "Hit"))

(event OnComponentBeginOverlap(WallDetector)
  (params (OverlappedComponent :type Primitive%20Component%20Object%20Reference) (OtherActor :type Actor%20Object%20Reference) (OtherComp :type Primitive%20Component%20Object%20Reference) (OtherBodyIndex :type Integer) (bFromSweep :type Boolean) (SweepResult :type Hit%20Result%20Structure%20%28by%20ref%29))
  (CallFunction|RotateCharacter))

(event OnComponentEndOverlap(FloorDetector)
  (params (OverlappedComponent :type Primitive%20Component%20Object%20Reference) (OtherActor :type Actor%20Object%20Reference) (OtherComp :type Primitive%20Component%20Object%20Reference) (OtherBodyIndex :type Integer))
  (CallFunction|RotateCharacter))

(event Custom|Hit
  (Class|BPIEnemyInterface|DamageTarget(Message) (stale OnComponentBeginOverlap(Box) OtherActor) 1.0 0.0))

(event EventDamageTarget
  (params (Amount :type Float%20%28double-precision%29) (HeartDropChance :type Float%20%28double-precision%29))
  (Variables|Default|SetHealth (- (Variables|Default|GetHealth) Amount))
  (if (<= (Variables|Default|GetHealth) 0.0)
    (CallFunction|Death HeartDropChance)))

(event EventTick
  (params (DeltaSeconds :type Float%20%28single-precision%29))
  (Pawn|Input|AddMovementInput (Transformation|GetActorForwardVector) 1.0 false))

(fn ConstructionScript)

(fn RotateCharacter
  (Transformation|SetActorRotation (Math|Rotator|CombineRotators (Transformation|GetActorRotation) "0.000000,180.000000,0.000000")))

(fn Death
  (params (HeartDropChance :type Float%20%28double-precision%29))
  (if (<= (Math|Random|RandomFloatinRange 0.0 1e+02) HeartDropChance)
    (Game|SpawnActorfromClass "/Game/Blueprints/BP_HealthPickup.BP_HealthPickup_C" (Math|Transform|MakeTransform (Transformation|GetWorldLocation (Variables|Default|GetPlane)) "0, 0, 0" "1.000000,1.000000,1.000000") "AlwaysSpawn" "MultiplyWithRoot" 0 0))
  (Actor|DestroyActor))