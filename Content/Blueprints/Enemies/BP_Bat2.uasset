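; BP_Bat2 is a bat enemy that bobs vertically and deals contact damage.
; A FlipFlop re-triggered on each Timeline finish alternates forward and reverse playback, lerping the root between its start height and a point above it.
; Box overlap with any BPI_EnemyInterface actor starts a looping timer that repeatedly sends DamageTarget until end overlap clears it.
; Incoming DamageTarget calls are forwarded to ACEnemyComponent.
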(event OnComponentBeginOverlap(Box)
  (params (OverlappedComponent :type Primitive%20Component%20Object%20Reference) (OtherActor :type Actor%20Object%20Reference) (OtherComp :type Primitive%20Component%20Object%20Reference) (OtherBodyIndex :type Integer) (bFromSweep :type Boolean) (SweepResult :type Hit%20Result%20Structure%20%28by%20ref%29))
  (if (Utilities|DoesObjectImplementInterface OtherActor "/Game/Blueprints/BPI_EnemyInterface.BPI_EnemyInterface_C")
    (Utilities|Time|SetTimerbyEvent (delegate Custom|Hit) 0.1 true)))

(event OnComponentEndOverlap(Box)
  (params (OverlappedComponent :type Primitive%20Component%20Object%20Reference) (OtherActor :type Actor%20Object%20Reference) (OtherComp :type Primitive%20Component%20Object%20Reference) (OtherBodyIndex :type Integer))
  (Utilities|Time|ClearTimerbyFunctionName 0 "Hit"))

(event Custom|Hit
  (Class|BPIEnemyInterface|DamageTarget(Message) (stale OnComponentBeginOverlap(Box) OtherActor) 1.0 0.0))

(event EventDamageTarget
  (params (Amount :type Float%20%28double-precision%29) (HeartDropChance :type Float%20%28double-precision%29))
  (Default|DamageEnemy (Variables|Default|GetAC_EnemyComponent) Amount))

(event EventBeginPlay
  (Variables|Default|SetInitialLocation (Transformation|GetWorldLocation (Variables|Default|GetDefaultSceneRoot)))
  (Utilities|FlowControl|FlipFlop :!label _label
    (:A
      (bind _alpha (Timeline|Timeline PlayFromStart)
        (:Update
          (Transformation|SetWorldLocation (Variables|Default|GetDefaultSceneRoot) (Math|Vector|MakeVector (.x (Variables|Default|GetInitialLocation)) (.y (Variables|Default|GetInitialLocation)) (Math|Float|Lerp (.z (Variables|Default|GetInitialLocation)) (+ (.z (Variables|Default|GetInitialLocation)) 2e+02) _alpha)) false false))
        (:Finished
          (goto _label))))
    (:B
      (Timeline|Timeline ReverseFromEnd))))

(fn ConstructionScript)