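; Bat enemy that bobs up and down above its starting position.
; BeginPlay stores the capsule location, then a timeline lerps its height between that point and a fixed offset above.
; A FlipFlop re-entered on each timeline finish alternates forward and reverse playback for an endless loop, printing debug strings on each switch.
; A RotateCharacter function applies a half-turn to the actor but is not called in this Blueprint.
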(event EventBeginPlay
  (Variables|Default|SetInitialLocation (Transformation|GetWorldLocation (Variables|Collision|GetCapsuleComponent)))
  (Utilities|FlowControl|FlipFlop :!label _label
    (:A
      (Development|PrintString "A")
      (bind _alpha (Timeline|Timeline PlayFromStart)
        (:Update
          (Transformation|SetRelativeLocation (Variables|Collision|GetCapsuleComponent) (Math|Vector|MakeVector (.x (Variables|Default|GetInitialLocation)) (.y (Variables|Default|GetInitialLocation)) (Math|Float|Lerp (.z (Variables|Default|GetInitialLocation)) (+ (.z (Variables|Default|GetInitialLocation)) 2e+02) _alpha)) false false))
        (:Finished
          (goto _label))))
    (:B
      (Development|PrintString "B")
      (Timeline|Timeline ReverseFromEnd))))

(fn ConstructionScript)

(fn RotateCharacter
  (Transformation|SetActorRotation (Math|Rotator|CombineRotators (Transformation|GetActorRotation) "0.000000,180.000000,0.000000")))