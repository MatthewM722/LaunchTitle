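; Actor component that gives enemies health and death handling.
; DamageEnemy subtracts damage from Health and calls Death once it reaches zero or below.
; Death reads drop chance and chain-damage state from the player's BP_Character, then rolls to spawn a BP_HealthPickup at the owner's location.
; The owner is destroyed only when chain damage is inactive; otherwise this component leaves it alive.
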(event Custom|Damage%20Enemy
  (params (Amount :type Float%20%28double-precision%29))
  (Variables|Default|SetHealth (- (Variables|Default|GetHealth) Amount))
  (if (<= (Variables|Default|GetHealth) 0.0)
    (CallFunction|Death)))

(event EventBeginPlay)

(event EventTick
  (params (DeltaSeconds :type Float%20%28single-precision%29)))

(fn Death
  (bind _asbp_character (Utilities|Casting|CastToBP_Character (Game|GetPlayerCharacter 0)))
  (LocalVariables|SetHeartDropChance (Variables|/Game/Player/BP_Character.BP_Character_C|GetHeartDropChance _asbp_character))
  (LocalVariables|SetChainDamageActive (Variables|/Game/Player/BP_Character.BP_Character_C|GetChainDamageActive _asbp_character))
  (if (<= (Math|Random|RandomFloatinRange 0.0 1e+02) (LocalVariables|GetHeartDropChance))
    (Game|SpawnActorfromClass "/Game/Blueprints/BP_HealthPickup.BP_HealthPickup_C" (Math|Transform|MakeTransform (Transformation|GetWorldLocation (Variables|/Script/Engine.Actor|GetRootComponent (Components|GetOwner))) "0, 0, 0" "1.000000,1.000000,1.000000") "AlwaysSpawn" "MultiplyWithRoot" 0 0))
  (if (not (LocalVariables|GetChainDamageActive))
    (Actor|DestroyActor (Components|GetOwner))))