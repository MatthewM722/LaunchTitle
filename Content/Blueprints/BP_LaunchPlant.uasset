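; BP_LaunchPlant is a plant that periodically becomes active and launches the player with a set Strength.
; On BeginPlay a looping timer calls Launch by function name, with a period of the launch delay plus the launch duration.
; Launch enables query-only collision on the box and shows three planes for the duration, then turns both off.
; The Interact event does the actual launch by calling LaunchPlayer on the player passed in.
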(event Custom|Launch
  (Collision|SetCollisionEnabled (Variables|Default|GetBox) "QueryOnly")
  (Rendering|SetVisibility (Variables|Default|GetPlane1) true false)
  (Utilities|FlowControl|Delay (Variables|Default|GetLaunchDuration))
  (Collision|SetCollisionEnabled (Variables|Default|GetBox) "NoCollision")
  (Rendering|SetVisibility (Variables|Default|GetPlane1) false false))

(event EventInteract
  (params (Player :type BP%20Character%20Object%20Reference))
  (Default|LaunchPlayer Player (Variables|Default|GetStrength)))

(event EventBeginPlay
  (CallFunction|BeginTimer))

(fn ConstructionScript)

(fn BeginTimer
  (bind _returnvalue (Utilities|Time|SetTimerbyFunctionName 0 "Launch" (+ (Variables|Default|GetLaunchDelayTimer) (Variables|Default|GetLaunchDuration)) true))
  (Variables|Default|SetTimerHandle _returnvalue))