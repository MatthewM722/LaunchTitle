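; BP_LevelLoader is a trigger actor that swaps streamed levels when something begins overlapping its Box component.
; The overlap, with no check on the overlapping actor, asynchronously loads and shows LevelToLoad, then asynchronously unloads LevelToUnload, both as soft level references.
; Debug messages then print both level names on screen.
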(event OnComponentBeginOverlap(Box)
  (params (OverlappedComponent :type Primitive%20Component%20Object%20Reference) (OtherActor :type Actor%20Object%20Reference) (OtherComp :type Primitive%20Component%20Object%20Reference) (OtherBodyIndex :type Integer) (bFromSweep :type Boolean) (SweepResult :type Hit%20Result%20Structure%20%28by%20ref%29))
  (Class|GameplayStatics|LoadStreamLevelbySoftObjectPtr (Variables|Default|GetLevelToLoad) true false)
  (Class|GameplayStatics|UnloadStreamLevelbySoftObjectPtr (Variables|Default|GetLevelToUnload) false)
  (Development|PrintString (Utilities|String|Append "Level Unloaded: " (Utilities|ToString(SoftObjectReference) (Variables|Default|GetLevelToUnload))) true true "(R=0.000000,G=0.660000,B=1.000000,A=1.000000)" 4.0)
  (Development|PrintString (Utilities|String|Append "Level Loaded: " (Utilities|ToString(SoftObjectReference) (Variables|Default|GetLevelToLoad))) true true "(R=0.000000,G=0.660000,B=1.000000,A=1.000000)" 4.0))

(fn ConstructionScript)